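; Demo actor for runtime mesh export that writes a static mesh to the project's Export folder on BeginPlay, printing supported formats and results.
; It implements MeshExportable, building sections from a CPU-accessible mesh with white vertex colors and a hierarchy node name.
; RuntimeMeshExporter pulls that data and writes the format picked by list index.
; An unwired import branch rebuilds scenes as procedural meshes with name-mapped materials; async import and export nodes are also unwired.
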(event `self.ReceiveBeginPlay`
  (bind _exportdelay (`self.ExportDelay`))
  (`|ExecutionSequence`
    (:`then_0`
      ;[1 1 1] Print Export Extensions
      (bind _formats (`RuntimeMeshImportExportLibrary.GetSupportedExtensionsExport`))
      (for (_array_element _array_index) _formats
        (bind (_id _description _fileextension) (break `AssimpExportFormat` _array_element))
        (`KismetSystemLibrary.PrintString` (`KismetStringLibrary.Concat_StrStr` (`KismetStringLibrary.Conv_IntToString` _array_index) ": " _id "     " _description "      " _fileextension) true true (struct :`G` 0.66 :`B` 1.0 :`A` 1.0) (`self.ExportFormatDelay`))))
    (:`then_1`
      (`KismetSystemLibrary.Delay` (`self.ExportFormatDelay`))
      (`|ExecutionSequence`
        (:`then_0`
          ;[1 1 1] Export
          (`KismetSystemLibrary.PrintString` "Exporting StaticMeshAsset" true true (struct :`G` 0.66 :`B` 1.0 :`A` 1.0) (`self.ExportDelay`))
          (bind _returnvalue (`|GenericCreateObject` "/Script/RuntimeMeshImportExport.RuntimeMeshExporter" self))
          ;;[1 1 1] See Interface "MeshExportable" implementation
          (`RuntimeMeshExporter.AddExportObject` _returnvalue self false "")
          (bind _formats_2 (`RuntimeMeshImportExportLibrary.GetSupportedExtensionsExport`))
          (bind (_id_2 _description_2 _fileextension_2) (break `AssimpExportFormat` (`|GetArrayItem` _formats_2 3)))
          (bind _result (`RuntimeMeshExporter.Export` _returnvalue (make `RuntimeMeshExportParam` false 0 false _id_2 (`KismetStringLibrary.Concat_StrStr` (`KismetSystemLibrary.GetProjectDirectory`) "/Export/ModernChair131" "." _fileextension_2) true (make `TransformCorrection` false false false "Plus_90"))))
          (bind (_bsuccess _exportlog _error _numobjectsskipped) (break `RuntimeMeshExportResult` _result))
          (`KismetSystemLibrary.PrintString` (`KismetStringLibrary.Concat_StrStr` "Export Done: " (select `bool` _bsuccess :`false` (`KismetStringLibrary.Concat_StrStr` "ERROR " _error) :`true` "SUCCESS") "    Num Objects Skipped: " (`KismetStringLibrary.Conv_IntToString` _numobjectsskipped)) true true (struct :`G` 0.66 :`B` 1.0 :`A` 1.0) _exportdelay)
          (`KismetSystemLibrary.PrintString` (`KismetStringLibrary.Concat_StrStr` "ExportLog:  \n" _exportlog) true true (struct :`R` 1.0 :`G` 0.405446 :`A` 1.0) _exportdelay))
        (:`then_2`
          ;[1 1 1] Demo Finish
          (`KismetSystemLibrary.Delay` (`self.ImportDelay`))
          (`KismetSystemLibrary.PrintString` "DONE" true true (struct :`G` 0.66 :`B` 1.0 :`A` 1.0) 5.0))))))

(fn `CreateColorArray`
  (params (Num :type Integer) (Color :type "Color Structure (by ref)"))
  (returns (Colors :type "Array of Color Structure"))
  (locals (L_Colors :type "Array of Color Structure"))
  (for _ (range 1 (+ Num 1))
    (`KismetArrayLibrary.Array_Add` (`local.L_Colors`) Color))
  (return (`local.L_Colors`)))

(fn `ExtractStaticMeshData`
  (params (forLod :type Integer :default 0) (bSkipLodNotValid :type Boolean :default false))
  (returns (outSectionData :type "Array of ExportableMeshSection Structure") (ReturnValue :type Boolean))
  (bind _toexport (`self.ToExport`))
  (`KismetArrayLibrary.Array_Clear` (`self.MeshSections`))
  (for _index (range (`StaticMesh.GetNumSections` _toexport forLod))
    (bind (_vertices _triangles _normals _uvs _tangents) (`KismetProceduralMeshLibrary.GetSectionFromStaticMesh` _toexport forLod _index)) ; Mesh must be marked as CPU ACCESSIBLE\nwithin the static mesh editor
    (`KismetArrayLibrary.Array_Add` (`self.MeshSections`) (make `ExportableMeshSection` (`KismetMathLibrary.MakeTransform` (0.0 0.0 0.0)) (`StaticMesh.GetMaterial` _toexport _index) _vertices _normals (`RuntimeMeshImportExportLibrary.ConvertProceduralMeshTangentToVector` _tangents) _uvs (`self.CreateColorArray` (`KismetArrayLibrary.Array_Length` _vertices) (make `Color` 255 255 255 255)) _triangles)))
  (return (`self.MeshSections`) true) ; MUST RETURN TRUE TO GET EXPORTED
)

(fn `GetHierarchicalNodeName`
  (returns (ReturnValue :type String))
  ;[1 1 1] Where the exported mesh shall be placed in the node hierarchy. Is only called when not overriden trough the Exporter::Add... functions
  (return "MyRoot.ParentNode.MyMesh"))

(fn `GetMeshData`
  (params (forLod :type Integer) (bSkipLodNotValid :type Boolean))
  (returns (outSectionData :type "Array of ExportableMeshSection Structure") (ReturnValue :type Boolean))
  (`self.ExtractStaticMeshData` forLod bSkipLodNotValid)
  (return (`self.GetStaticMeshData`) true) ; MUST RETURN TRUE TO GET EXPORTED
)

(fn `GetStaticMeshData`
  (returns (outSectionData :type "Array of ExportableMeshSection Structure"))
  (return (`self.MeshSections`)) ; MUST RETURN TRUE TO GET EXPORTED
)

(fn `UserConstructionScript`)