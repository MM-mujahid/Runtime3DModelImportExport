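; Mesh converter prototype, apparently from a Runtime Mesh Exporter demo, that implements MeshExportable to supply geometry for file export.
; ImportFBX only stores a path; the export chain is disconnected, and BeginPlay just waits.
; ExtractStaticMeshData builds white-vertex-colored sections from the CPU-accessible ToExport mesh.
; GetMeshData runs it but returns GetStaticMeshData instead, an unfinished stub that imports the file and outputs no sections.
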(event `self.ReceiveBeginPlay`
  (`|ExecutionSequence`
    (:`then_1`
      (`KismetSystemLibrary.Delay` (`self.ExportFormatDelay`))
      (`|ExecutionSequence`))))

(event `ImportFBX`
  (params (filePath :type String))
  ;[1 1 1] Import
  (set `self.FilePath` filePath))

(fn `CreateColorArray`
  (params (Num :type Integer) (Color :type "Color Structure (by ref)"))
  (returns (Colors :type "Array of Color Structure"))
  (locals (L_Colors :type "Array of Color Structure"))
  (for _ (range 1 (+ Num 1))
    (`KismetArrayLibrary.Array_Add` (`local.L_Colors`) Color))
  (return (`local.L_Colors`)))

(fn `ExtractStaticMeshData`
  (params (forLod :type Integer :default 0) (bSkipLodNotValid :type Boolean :default false))
  (returns (outSectionData :type "Array of ExportableMeshSection Structure") (ReturnValue :type Boolean))
  (bind _toexport (`self.ToExport`))
  (`KismetArrayLibrary.Array_Clear` (`self.MeshSections`))
  (for _index (range (`StaticMesh.GetNumSections` _toexport forLod))
    (bind (_vertices _triangles _normals _uvs _tangents) (`KismetProceduralMeshLibrary.GetSectionFromStaticMesh` _toexport forLod _index)) ; Mesh must be marked as CPU ACCESSIBLE\nwithin the static mesh editor
    (`KismetArrayLibrary.Array_Add` (`self.MeshSections`) (make `ExportableMeshSection` (`KismetMathLibrary.MakeTransform` (0.0 0.0 0.0)) (`StaticMesh.GetMaterial` _toexport _index) _vertices _normals (`RuntimeMeshImportExportLibrary.ConvertProceduralMeshTangentToVector` _tangents) _uvs (`self.CreateColorArray` (`KismetArrayLibrary.Array_Length` _vertices) (make `Color` 255 255 255 255)) _triangles)))
  (return (`self.MeshSections`) true) ; MUST RETURN TRUE TO GET EXPORTED
)

(fn `GetHierarchicalNodeName`
  (returns (ReturnValue :type String))
  ;[1 1 1] Where the exported mesh shall be placed in the node hierarchy. Is only called when not overriden trough the Exporter::Add... functions
  (return "MyRoot.ParentNode.MyMesh"))

(fn `GetMeshData`
  (params (forLod :type Integer) (bSkipLodNotValid :type Boolean))
  (returns (outSectionData :type "Array of ExportableMeshSection Structure") (ReturnValue :type Boolean))
  (`self.ExtractStaticMeshData` forLod bSkipLodNotValid)
  (return (`self.GetStaticMeshData`) true) ; MUST RETURN TRUE TO GET EXPORTED
)

(fn `GetStaticMeshData`
  (returns (outSectionData :type "Array of ExportableMeshSection Structure"))
  (bind _result (`RuntimeMeshImportExportLibrary.ImportScene` (`self.FilePath`) (`KismetMathLibrary.MakeTransform` (0.0 0.0 0.0))))
  (bind (_bsuccess _meshinfos) (break `RuntimeMeshImportResult` _result))
  (if _bsuccess
    (for _array_element _meshinfos
      (return) ; MUST RETURN TRUE TO GET EXPORTED
    )))

(fn `UserConstructionScript`)